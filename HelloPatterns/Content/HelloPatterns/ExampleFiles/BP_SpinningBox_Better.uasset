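; BP_SpinningBox_Better is an example Blueprint from HelloPatterns for a box that spins around its yaw axis.
; Tick adds a fixed relative yaw step to StaticMeshBox each frame, independent of delta time, and subtracts a full turn once yaw reaches 360.
; A construction script also copies a RotationRate variable into a RotatingMovement component, so both manual and component-driven rotation appear, alongside a second, empty construction script.
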(event `self.ReceiveTick`
  (params (DeltaSeconds :type "Float (single-precision)"))
  (bind (_relativerotation_roll _relativerotation_pitch _relativerotation_yaw) (`KismetMathLibrary.BreakRotator` (`SceneComponent.RelativeRotation` (`self.StaticMesh_Box`))))
  (`SceneComponent.K2_AddRelativeRotation` (`self.StaticMesh_Box`) (struct :`Yaw` 2.0) false false)
  (if (>= _relativerotation_yaw 360.0)
    (`SceneComponent.K2_SetRelativeRotation` (`self.StaticMesh_Box`) (`KismetMathLibrary.MakeRotator` 0.0 0.0 (- _relativerotation_yaw 360.0)) false false)))

(fn `UserConstructionScript`)

(fn `UserConstructionScript`
  (set `RotatingMovementComponent.RotationRate` (`self.Rotation Rate`) (`self.RotatingMovement`)))