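; BP_EliteUnit is an RTS elite unit pawn that takes move, stop and attack commands.
; On possession it caches its AIC_EliteUnit controller, and move or stop commands write the target or current location to that controller's MoveToLocation blackboard key.
; Attacks run a debug-drawn visibility trace to the target and apply fixed damage on a direct hit, otherwise printing that line of sight is missing.
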(event `self.ReceivePossessed`
  (params (NewController :type "Controller Object Reference"))
  (bind _asaic_elite_unit (cast `/Game/RTS/Blueprints/AIC_EliteUnit` NewController))
  (set `self.AIEliteController` _asaic_elite_unit))

(event `self.SetMoveLocation`
  (params (targetLocation :type "Vector Structure"))
  (set `self.MoveToLocation` targetLocation)
  (`BlackboardComponent.SetValueAsVector` (`AIBlueprintHelperLibrary.GetBlackboard` (`self.AIEliteController`)) "MoveToLocation" (`self.MoveToLocation`)))

(event `self.StopMoving`
  (set `self.MoveToLocation` (`self.K2_GetActorLocation`))
  (`BlackboardComponent.SetValueAsVector` (`AIBlueprintHelperLibrary.GetBlackboard` (`self.AIEliteController`)) "MoveToLocation" (`self.MoveToLocation`)))

(event `self.AttackTarget`
  (params (target :type "Object Object Reference"))
  (bind _asactor (cast `Actor` target))
  (bind _outhit (`KismetSystemLibrary.LineTraceSingle` :`Start` (`self.K2_GetActorLocation`) :`End` (`self.K2_GetActorLocation` _asactor) :`TraceChannel` "TraceTypeQuery1" :`DrawDebugType` "ForDuration"))
  (bind (_bblockinghit _binitialoverlap _time _distance _location _impactpoint _normal _impactnormal _physmat _hitactor) (`GameplayStatics.BreakHitResult` _outhit))
  (if (== _hitactor target)
    (`GameplayStatics.ApplyDamage` _hitactor 100.0)
    (else
      (`KismetSystemLibrary.PrintString` "No Line of Sight"))))

(fn `UserConstructionScript`)